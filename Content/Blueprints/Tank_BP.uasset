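; Tank Blueprint with a player-aimed camera rig and barrel and turret components.
; On BeginPlay it passes the Barrel and Turret components to SetBarrelReference.
; Aim axis inputs yaw the AzemuthGimbal and pitch the SpringArm, scaled by AimSensitivity and world delta time for frame-rate independence.
; The construction script assigns the barrel's mesh and material and zeroes its relative location.
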(event `self.ReceiveBeginPlay`
  (`self.SetBarrelReference` (`self.Barrel`) (`self.Turret`)))

(event `InputAxis|AimAzimuth`
  (params (AxisValue :type "Float (single-precision)"))
  ;[1 1 1] View Controls
  (`SceneComponent.K2_AddLocalRotation` (`self.Azemuth Gimbal`) (`KismetMathLibrary.MakeRotator` 0.0 0.0 (* AxisValue (`GameplayStatics.GetWorldDeltaSeconds`) (`self.Aim Sensitivity`))) false false))

(event `InputAxis|AimElevation`
  (params (AxisValue :type "Float (single-precision)"))
  ;[1 1 1] View Controls
  (`SceneComponent.K2_AddLocalRotation` (`self.SpringArm`) (`KismetMathLibrary.MakeRotator` 0.0 (* AxisValue (`GameplayStatics.GetWorldDeltaSeconds`) (`self.Aim Sensitivity`))) false false))

(fn `UserConstructionScript`
  (bind _barrel (`self.Barrel`))
  (`StaticMeshComponent.SetStaticMesh` _barrel "/Game/Tank/tank_fbx_Barrel.tank_fbx_Barrel")
  (`PrimitiveComponent.SetMaterial` _barrel 0 "/Game/Materials/FlatLand.FlatLand")
  (`SceneComponent.K2_SetRelativeLocation` _barrel (0.0 0.0 0.0) false false))